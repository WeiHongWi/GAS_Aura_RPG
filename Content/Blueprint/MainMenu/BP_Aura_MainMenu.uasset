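; BP_Aura_MainMenu is an actor for the main menu scene that sets up the menu and animates its Fire component.
; On BeginPlay it stores the fire's location, plays menu music, and shows the BP_MainMenu widget with UI-only input and a mouse cursor.
; Each Tick, UpdateTime advances a timer that resets after one sine period, driving a vertical bob of the fire around its starting position.
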(event `self.ReceiveBeginPlay`
  (bind _returnvalue (`GameplayStatics.GetPlayerController` 0))
  (set `self.InitialLocation` (`SceneComponent.K2_GetComponentLocation` (`self.Fire`)))
  (`GameplayStatics.PlaySound2D` "/Game/Assets/Sounds/Music/Music_MainMenu.Music_MainMenu" 1.0 1.0 0.0 null null)
  (bind _returnvalue_2 (`|CreateWidget` "/Game/Blueprint/MainMenu/BP_MainMenu.BP_MainMenu_C"))
  (`UserWidget.AddToViewport` _returnvalue_2 0)
  (`WidgetBlueprintLibrary.SetInputMode_UIOnlyEx` _returnvalue _returnvalue_2)
  (set `PlayerController.bShowMouseCursor` true _returnvalue))

(event `self.ReceiveTick`
  (params (DeltaSeconds :type "Float (single-precision)"))
  (`self.UpdateTime` DeltaSeconds)
  (`SceneComponent.K2_SetWorldLocation` (`self.Fire`) (+ (`self.InitialLocation`) (`KismetMathLibrary.MakeVector` 0.0 0.0 (* (`KismetMathLibrary.Sin` (`self.Time`)) (`self.Amplitude`)))) false false))

(fn `UpdateTime`
  (params (A :type "Float (double-precision)"))
  (bind _returnvalue (+ A (`self.Time`)))
  (set `self.Updating Time` _returnvalue)
  (if (< _returnvalue 6.28318)
    (set `self.Time` (`self.Updating Time`))
    (else
      (set `self.Time` 0.0))))

(fn `UserConstructionScript`)