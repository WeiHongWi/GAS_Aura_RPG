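; BP_FirePillar is a fire pillar actor whose point light varies in intensity to act as a flame.
; On BeginPlay it makes a random pick intended to choose between two flame timelines, each scaling BaseIntensity onto the light.
; The random range of 1 to 2 mismatches switch cases 0 and 1, so only the second timeline can start, or neither.
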(event `self.ReceiveBeginPlay`
  (`self.RandomChoose`))

(event `RandomChoose`
  (switch `int` (`KismetMathLibrary.RandomIntegerInRange` 1 2)
    (:`0`
      (`self.FlameTimeline_1`))
    (:`1`
      (`self.FlameTimeline_2`))))

(event `FlameTimeline_1`
  (bind (_direction _newtrack_0) (`Timeline|FlameTimeline`)
    (:`Update`
      (`LightComponent.SetIntensity` (`self.PointLight`) (* _newtrack_0 (`self.BaseIntensity`))))))

(event `FlameTimeline_2`
  (bind (_direction _newtrack_0) (`Timeline|FlameTimeline2`)
    (:`Update`
      (`LightComponent.SetIntensity` (`self.PointLight`) (* _newtrack_0 (`self.BaseIntensity`))))))

(fn `UserConstructionScript`)