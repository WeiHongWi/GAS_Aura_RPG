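; Gameplay ability for Arcane Shards, which shows a targeting magic circle and, on input press, bursts shards at ground points around the spot under the mouse.
; A spawned BP_PointCollection supplies the points, and a montage gameplay event hides the circle and starts a looping timer.
; Each tick radially damages live players near the next point except the caster, fires a gameplay cue and commits cost.
; After the last point it destroys the collection, commits cooldown and ends.
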(event `self.K2_ActivateAbility`
  (`|ExecutionSequence`
    (:`then_0`
      (message `CombatInterface.ShowMagicCircle` (`self.GetAvatarActorFromActorInfo`) "/Game/Assets/MagicCircles/M_MagicCircle_1.M_MagicCircle_1"))
    (:`then_1`
      (`AbilityTask_WaitInputPress.WaitInputPress` false
        (:`OnPress`
          (bind (_asynctaskproxy _data) (`TargetDataUnderMouse.CreateTargetDataUnderMouse`)
            (:`ValidData`
              (bind (_bblockinghit _binitialoverlap _time _distance _location _impactpoint) (`GameplayStatics.BreakHitResult` (`AbilitySystemBlueprintLibrary.GetHitResultFromTargetData` _data)))
              (bind _returnvalue (`|SpawnActorFromClass` "/Game/Blueprint/AbilitySystem/GameplayAbility/Arcane/ArcaneShard/BP_PointCollection.BP_PointCollection_C" (`KismetMathLibrary.MakeTransform` _impactpoint) "AlwaysSpawn" "MultiplyWithRoot" null null))
              (set `self.PointCollection` _returnvalue)
              (set `self.GroundPoints` (`PointCollectionActor.GetGroundPoints` _returnvalue _impactpoint (`self.Num Points`) 10.0))
              (`AbilityTask_PlayMontageAndWait.CreatePlayMontageAndWaitProxy` "None" "/Game/Assets/Characters/Aura/Animations/Abilities/AM_ArcaneShards.AM_ArcaneShards"
                (:`then`
                  (`AbilityTask_WaitGameplayEvent.WaitGameplayEvent` (struct :`TagName` "Event.Montage.ArcaneShard") null
                    (:`EventReceived`
                      (bind _returnvalue_2 (`KismetSystemLibrary.K2_SetTimerDelegate` (delegate `TriggerArcaneShard`) (`self.Time`) true))
                      (set `self.TimerHandleShard` _returnvalue_2)
                      (message `CombatInterface.HideMagicCircle` (`self.GetAvatarActorFromActorInfo`)))))))))))))

(event `self.K2_OnEndAbility`
  (params (bWasCancelled :type Boolean)))

(event `TriggerArcaneShard`
  (bind _returnvalue (`self.GetAvatarActorFromActorInfo`))
  (if (< (`self.Count`) (`self.Num Points`))
    (set `self.PointLocation` (`SceneComponent.K2_GetComponentLocation` (`|GetArrayItem` (`self.GroundPoints`) (`self.Count`))))
    (bind _outoverlappingactors (`AuraAbilitySystemLibrary.GetLivePlayersWithinRadius` _returnvalue (`|MakeArray` _returnvalue) (`self.RadialDamageOuterRadius`) (`self.PointLocation`)))
    (bind _output_get (set `self.OverlappingActors` _outoverlappingactors))
    (for _array_element _output_get
      (`AuraAbilitySystemLibrary.ApplyDamageEffect` (`self.InitialDamageEffect` _array_element (`self.PointLocation`))))
    (`/Engine/EditorBlueprintResources/StandardMacros.IncrementInt` (`self.Count`)
      (:`  `
        (`self.K2_ExecuteGameplayCueWithParams` (struct :`TagName` "GameplayCue.ArcaneShard") (`AbilitySystemBlueprintLibrary.MakeGameplayCueParameters` 0.0 0.0 (struct) (struct) (struct) (struct) (struct) (`self.PointLocation`)))
        (`self.K2_CommitAbilityCost` false)))
    (else
      (`KismetSystemLibrary.K2_ClearAndInvalidateTimerHandle` (`self.TimerHandleShard`))
      (`KismetSystemLibrary.Delay` 0.0)
      (`Actor.K2_DestroyActor` (`self.PointCollection`))
      (`self.K2_CommitAbilityCooldown` false)
      (`self.K2_EndAbility`))))