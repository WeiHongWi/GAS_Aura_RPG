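; BP_FireBall is a Fire Blast projectile that flies out, returns toward a given actor and explodes near it.
; On authority, two chained timelines lerp it forward to an apex, then back to ReturningActor's live location.
; Once within ExplodeRange it calls OnHit, applies radial damage effects with knockback and death impulse to live players in OuterRadius except its owner, then destroys itself.
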(event `self.StartOutgoingTimeline`
  (bind (_returnvalue_roll _returnvalue_pitch _returnvalue_yaw) (`KismetMathLibrary.BreakRotator` (`KismetMathLibrary.MakeRotFromX` (`self.ImpulseDirection`))))
  (bind _array (`|MakeArray` (`self.GetOwner`)))
  (`/Engine/EditorBlueprintResources/ActorMacros.Switch Has Authority`
    (:`Authority`
      (set `self.InitialLocation` (`self.K2_GetActorLocation`))
      (set `self.ApexLocation` (+ (`self.InitialLocation`) (* (`self.GetActorForwardVector`) (`self.TargetDistance`))))
      (bind (_direction _newtrack_0) (`Timeline|Timeline`)
        (:`Update`
          (`self.K2_SetActorLocation` (`KismetMathLibrary.VLerp` (`self.InitialLocation`) (`self.ApexLocation`) _newtrack_0)))
        (:`Finished`
          (bind (_direction_2 _newtrack_0_2) (`Timeline|Returning Back`)
            (:`Update`
              (`self.K2_SetActorLocation` (`KismetMathLibrary.VLerp` (`self.ApexLocation`) (`self.K2_GetActorLocation` (`self.ReturningActor`)) _newtrack_0_2))
              (bind _returnvalue (`self.IsExplodeRange`))
              (if _returnvalue
                (`self.OnHit`)
                (`AuraAbilitySystemLibrary.SetIsRadialDamageEffectParams` (`self.ExplosionDamageEffectParams`) true (`self.InnerRadius`) (`self.OuterRadius`) (`self.K2_GetActorLocation`))
                (`KismetArrayLibrary.Array_Add` _array self)
                (bind _outoverlappingactors (`AuraAbilitySystemLibrary.GetLivePlayersWithinRadius` self _array (`self.OuterRadius`) (`self.K2_GetActorLocation`)))
                (bind _output_get (set `self.OvelappingActor` _outoverlappingactors))
                (for _array_element _output_get
                  (`AuraAbilitySystemLibrary.SetTargetASCParams` (`self.ExplosionDamageEffectParams`) (`AbilitySystemBlueprintLibrary.GetAbilitySystemComponent` _array_element))
                  (set `self.ImpulseDirection` (- (`self.K2_GetActorLocation` _array_element) (`self.K2_GetActorLocation`)))
                  (`AuraAbilitySystemLibrary.SetKnockbackDirectionParams` (`self.ExplosionDamageEffectParams`) (`KismetMathLibrary.GetForwardVector` (`KismetMathLibrary.MakeRotator` _returnvalue_roll 0.0 _returnvalue_yaw)) 800.0)
                  (`AuraAbilitySystemLibrary.SetDeathImpulseDirectionParams` (`self.ExplosionDamageEffectParams`) (`self.ImpulseDirection`) 600.0)
                  (`AuraAbilitySystemLibrary.ApplyDamageEffect` (`self.ExplosionDamageEffectParams`)))
                (`self.K2_DestroyActor`)))))))))

(event `self.ReceiveBeginPlay`)

(fn `IsExplodeRange`
  (returns (ReturnValue :type Boolean))
  (return (<= (`KismetMathLibrary.VSize` (- (`self.K2_GetActorLocation`) (`self.K2_GetActorLocation` (`self.ReturningActor`)))) (`self.ExplodeRange`))))

(fn `UserConstructionScript`)