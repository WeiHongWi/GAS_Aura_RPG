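; Enemy melee attack gameplay ability that faces the avatar toward its combat target and plays a random attack montage.
; A gameplay event matching the montage's tag triggers a small radius check at the socket location for that attack, damaging live non-friendly players and triggering their blood effect.
; Any hit fires a MeleeAttack gameplay cue, and the ability ends after the hit check or when the montage finishes or is interrupted.
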(event `self.K2_ActivateAbility`
  (bind _returnvalue (`self.GetAvatarActorFromActorInfo`))
  (bind _returnvalue_2 (`self.GetAvatarActorFromActorInfo`))
  (bind _returnvalue_3 (`self.GetAvatarActorFromActorInfo`))
  (bind (_tagmontage_montage _tagmontage_montagetag) (break `TagMontage` (`self.TagMontage`)))
  (set `self.HasHitTarget` false)
  (bind _returnvalue_4 (message `CombatInterface.GetCombatTarget` _returnvalue_3))
  (bind _ascombat_interface (cast `CombatInterface` _returnvalue_3))
  (`CombatInterface.UpdateFacingTarget` _ascombat_interface (`Actor.K2_GetActorLocation` _returnvalue_4))
  (bind _returnvalue_5 (message `CombatInterface.GetAttackMontages` (`self.GetAvatarActorFromActorInfo`)))
  (bind _returnvalue_6 (`KismetArrayLibrary.Array_Length` _returnvalue_5))
  (bind _output_get (set `self.TagMontage` (`|GetArrayItem` _returnvalue_5 (`KismetMathLibrary.RandomIntegerInRange` 0 (- _returnvalue_6 1)))))
  (if (> _returnvalue_6 0)
    (bind (_montage _montagetag _sockettag) (break `TagMontage` _output_get))
    (`AbilityTask_PlayMontageAndWait.CreatePlayMontageAndWaitProxy` "None" _montage
      (:`then`
        (`AbilityTask_WaitGameplayEvent.WaitGameplayEvent` _montagetag null
          (:`EventReceived`
            (bind _returnvalue_7 (message `CombatInterface.GetWeaponTipSocketLocation` _returnvalue _sockettag))
            (set `self.WeaponSocketLocation` _returnvalue_7)
            (bind _outoverlappingactors (`AuraAbilitySystemLibrary.GetLivePlayersWithinRadius` _returnvalue (`|MakeArray` _returnvalue) 50.0 _returnvalue_7))
            (for _array_element _outoverlappingactors
              (if (not (`AuraAbilitySystemLibrary.IsFriend` (`self.GetAvatarActorFromActorInfo`) _array_element))
                (`self.CauseDamage` _array_element)
                (set `self.HasHitTarget` true)
                (message `CombatInterface.GetBloodEffect` _array_element)))
            (if (`self.HasHitTarget`)
              (bind _returnvalue_8 (message `CombatInterface.GetCombatTarget` _returnvalue_2))
              (`self.K2_ExecuteGameplayCueWithParams` (struct :`TagName` "GameplayCue.MeleeAttack") (`AbilitySystemBlueprintLibrary.MakeGameplayCueParameters` 0.0 0.0 (struct) (struct) (struct) (`BlueprintGameplayTagLibrary.MakeGameplayTagContainerFromTag` _tagmontage_montagetag) (struct) (`self.WeaponSocketLocation`) (0.0 0.0 0.0) null _returnvalue_2 _returnvalue_8)))
            (`self.K2_EndAbility`))))
      (:`OnCompleted`
        (`self.K2_EndAbility` :!label _label))
      (:`OnInterrupted`
        (goto _label))
      (:`OnCancelled`
        (goto _label)))
    (else
      (`self.K2_EndAbility`))))