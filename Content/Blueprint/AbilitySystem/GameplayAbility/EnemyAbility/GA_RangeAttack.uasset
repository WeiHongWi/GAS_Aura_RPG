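; GA_RangeAttack is an enemy gameplay ability for a ranged attack on the avatar's combat target.
; On activation it turns the avatar toward the target and plays a random attack montage, ending immediately if none exist.
; A gameplay event matching that montage's weapon tag triggers SpawnProjectile at the target's current location, re-read at that moment.
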(event `self.K2_ActivateAbility`
  (bind _returnvalue (`self.GetAvatarActorFromActorInfo`))
  (bind _returnvalue_2 (message `CombatInterface.GetCombatTarget` _returnvalue))
  (bind _ascombat_interface (cast `CombatInterface` _returnvalue))
  (bind _returnvalue_3 (`Actor.K2_GetActorLocation` _returnvalue_2))
  (set `self.TargetLocation` _returnvalue_3)
  (`CombatInterface.UpdateFacingTarget` _ascombat_interface _returnvalue_3)
  (bind _returnvalue_4 (message `CombatInterface.GetAttackMontages` (`self.GetAvatarActorFromActorInfo`)))
  (bind _returnvalue_5 (`KismetArrayLibrary.Array_Length` _returnvalue_4))
  (if (> _returnvalue_5 0)
    (bind _output_get (set `self.TargetToProjectile` (`|GetArrayItem` _returnvalue_4 (`KismetMathLibrary.RandomIntegerInRange` 0 (- _returnvalue_5 1)))))
    (bind (_montage _weapontag) (break `TagMontage` _output_get))
    (`AbilityTask_PlayMontageAndWait.CreatePlayMontageAndWaitProxy` "None" _montage
      (:`then`
        (`AbilityTask_WaitGameplayEvent.WaitGameplayEvent` _weapontag null
          (:`EventReceived`
            (message `CombatInterface.GetWeaponTipSocketLocation` (`self.GetAvatarActorFromActorInfo`) _weapontag)
            (bind _returnvalue_6 (message `CombatInterface.GetCombatTarget` (`self.GetAvatarActorFromActorInfo`)))
            (`self.SpawnProjectile` (`Actor.K2_GetActorLocation` _returnvalue_6))))))
    (else
      (`self.K2_EndAbility`))))