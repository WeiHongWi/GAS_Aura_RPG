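; Enemy summon gameplay ability that spawns random AI-controlled minions at shuffled spawn locations, using a shaman summon montage.
; On activation it plays ground Niagara effects at every location, then starts the montage and an attack-tag event wait.
; A delayed loop on the wait's immediate Then pin, not its received event, staggers the spawns.
; Each spawn raises the avatar's minion count, and its destruction lowers it.
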(event `self.K2_ActivateAbility`
  (bind _returnvalue (`self.GetAvatarActorFromActorInfo`))
  (bind _returnvalue_2 (`self.GetSpawnLocation`))
  (bind _output_get (set `self.SpawnLocations` _returnvalue_2))
  (`KismetArrayLibrary.Array_Shuffle` _output_get)
  (for _array_element _output_get
    (`NiagaraFunctionLibrary.SpawnSystemAtLocation` "/Game/Assets/Effects/Combat/NS_GroundSummon.NS_GroundSummon" _array_element))
  (`AbilityTask_PlayMontageAndWait.CreatePlayMontageAndWaitProxy` "None" "/Game/Assets/Enemies/Shaman/Animations/Shaman_Summon_Montage.Shaman_Summon_Montage"
    (:`then`
      (`AbilityTask_WaitGameplayEvent.WaitGameplayEvent` (struct :`TagName` "Montage.Attack.1") null
        (:`then`
          (if (< (`self.Index`) (`KismetArrayLibrary.Array_Length` _output_get)) :!label _label
            (bind _returnvalue_3 (`self.GetRandomMinion`))
            (bind _returnvalue_4 (`|SpawnActorFromClass` _returnvalue_3 (`KismetMathLibrary.MakeTransform` (+ (`|GetArrayItem` (`self.SpawnLocations`) (`self.Index`)) (0.0 0.0 70.0)) (`KismetMathLibrary.FindLookAtRotation` (`Actor.K2_GetActorLocation` _returnvalue) (`Actor.GetActorForwardVector` _returnvalue))) "AlwaysSpawn" "MultiplyWithRoot" null null))
            (add `Actor.OnDestroyed` _returnvalue_4 (delegate `OnDestroyed_Event`))
            (`Pawn.SpawnDefaultController` _returnvalue_4)
            (message `CombatInterface.IncreaseMinionCount` (`self.GetAvatarActorFromActorInfo`) 1)
            (`/Engine/EditorBlueprintResources/StandardMacros.IncrementInt` (`self.Index`)
              (:`  `
                (`KismetSystemLibrary.Delay` 0.2)
                (goto _label)))))))))

(event `OnDestroyed_Event`
  (params (DestroyedActor :type "Actor Object Reference"))
  (message `CombatInterface.IncreaseMinionCount` (`self.GetAvatarActorFromActorInfo`) -1))